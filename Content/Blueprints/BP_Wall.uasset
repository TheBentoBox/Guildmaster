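; BP_Wall is a wall actor that builds itself from a 3D grid of static mesh blocks when scaled.
; The construction script adds each axis's scale change from 1 to stored ScaleX/Y/Z totals, then resets actor scale to 1, so meshes tile without stretching.
; Nested loops over the floored totals add components at 100-unit spacing, skipping the origin cell.
; The event graph has no runtime logic.
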(event EventBeginPlay)

(event EventActorBeginOverlap
  (params (OtherActor :type Actor%20Object%20Reference)))

(event EventTick
  (params (DeltaSeconds :type Float%20%28single-precision%29)))

(fn ConstructionScript
  (bind _returnvalue (Transformation|GetActorScale3D))
  (bind (_x _y _z) (Math|Vector|BreakVector _returnvalue))
  ;[1 1 1] Dynamically add wall meshes based on scale
  (Variables|Default|SetScaleX (- (+ (Variables|Default|GetScaleX) _x) 1.0))
  (Variables|Default|SetScaleY (- (+ (Variables|Default|GetScaleY) _y) 1.0))
  (Variables|Default|SetScaleZ (- (+ _z (Variables|Default|GetScaleZ)) 1.0))
  (Transformation|SetActorScale3D "1.000000,1.000000,1.000000")
  (for _index (range 0 (Math|Float|Floor (Variables|Default|GetScaleX)))
    (for _index_2 (range 0 (Math|Float|Floor (Variables|Default|GetScaleY)))
      (for _index_3 (range 0 (Math|Float|Floor (Variables|Default|GetScaleZ)))
        (if (Math|Boolean|ORBoolean (!= _index 0) (!= _index_2 0) (!= _index_3 0))
          (AddComponent|AddStaticMeshComponent false (Math|Conversions|ToTransform(Vector) (* (Math|Vector|MakeVector (Math|Conversions|ToFloat(Integer) _index) (Math|Conversions|ToFloat(Integer) _index_2) (Math|Conversions|ToFloat(Integer) _index_3)) 100))))))))