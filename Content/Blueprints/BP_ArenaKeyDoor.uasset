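; Arena key door Blueprint that slides open from its start location once a trigger volume holds no Slime actors.
; Activate, also called on BeginPlay when IsActive is set, queries the volume and plays a timeline only if it is clear.
; The timeline moves the door along MoveOffset without sweeping, then destroys the trigger volume.
; It has no closing path, and its sound node never runs.
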(event EventActivate
  ;[1 1 1] Listens for code event and plays open/close timeline
  (if (== (Utilities|Array|Length (Collision|GetOverlappingActors (Variables|Default|GetTrigger%20Volume%20To%20Query) "/Game/Blueprints/Character/Slime/Slime.Slime_C" :!class /Script/Engine.Actor)) 0)
    (bind _open_amount (Timeline|Door%20Open%20Timeline Play)
      (:Update
        (Transformation|SetActorLocation (+ (* (Variables|Default|GetMove%20Offset) _open_amount) (Variables|Default|GetInitial%20Location)) false false))
      (:Finished
        (Actor|DestroyActor (Variables|Default|GetTrigger%20Volume%20To%20Query))))))

(event EventBeginPlay
  ;[1 1 1] Grab initial rotation for relative swing animation
  (Variables|Default|SetInitial%20Location (Transformation|GetActorLocation))
  (if (Variables|Default|GetIsActive)
    (CallFunction|Activate)))

(fn ConstructionScript
  (|CallParentFunction))