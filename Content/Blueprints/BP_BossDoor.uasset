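; Boss door Blueprint with two hinged leaves that swing open once all four of its locks are active.
; BeginPlay caches the world rotations of the left and right hinge arrows.
; Activate checks the locks, sets IsLocked to true, destroys the lock actors and plays a timeline.
; The timeline yaws the two hinges in opposite directions from their cached rotations.
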(event EventBeginPlay
  ;[1 1 1] Get rotation of door hinge arrows
  (Variables|Default|SetInitial%20Left%20Rotation (Transformation|GetWorldRotation (Variables|Default|GetLeftArrow)))
  (Variables|Default|SetInitial%20Right%20Rotation (Transformation|GetWorldRotation (Variables|Default|GetRightArrow))))

(event EventActivate
  ;[1 1 1] Check for sockets being filled then animate open
  (if (Math|Boolean|ANDBoolean (Variables|/Game/Blueprints/BP_Activatable.BP_Activatable_C|GetIsActive (Variables|Default|GetLock1)) (Variables|/Game/Blueprints/BP_Activatable.BP_Activatable_C|GetIsActive (Variables|Default|GetLock2)) (Variables|/Game/Blueprints/BP_Activatable.BP_Activatable_C|GetIsActive (Variables|Default|GetLock3)) (Variables|/Game/Blueprints/BP_Activatable.BP_Activatable_C|GetIsActive (Variables|Default|GetLock4)))
    (Variables|Default|SetIsLocked true)
    (Actor|DestroyActor (Variables|Default|GetLock1))
    (Actor|DestroyActor (Variables|Default|GetLock2))
    (Actor|DestroyActor (Variables|Default|GetLock3))
    (Actor|DestroyActor (Variables|Default|GetLock4))
    (bind _door_angle (Timeline|Door%20Swing%20Timeline Play)
      (:Update
        (Transformation|SetWorldRotation (Variables|Default|GetLeftArrow) (Math|Rotator|CombineRotators (Variables|Default|GetInitial%20Left%20Rotation) (Math|Rotator|MakeRotator 0.0 0.0 (* _door_angle -6e+01))) false false)
        (Transformation|SetWorldRotation (Variables|Default|GetRightArrow) (Math|Rotator|CombineRotators (Variables|Default|GetInitial%20Right%20Rotation) (Math|Rotator|MakeRotator 0.0 0.0 (* _door_angle 6e+01))) false false)))))

(fn ConstructionScript
  (|CallParentFunction))