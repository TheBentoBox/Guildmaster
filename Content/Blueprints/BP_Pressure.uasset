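; BP_Pressure is a pressure plate that toggles on while objects rest on it and off when it is clear.
; Box begin and end overlaps share one check that re-queries overlapping physics bodies, dynamic objects, pawns and destructibles, calling Toggle only when IsActive must change.
; The Activate event teleports the plate slightly below its BeginPlay location when active and restores it when inactive.
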(event OnComponentBeginOverlap(Box)
  (params (OtherActor :type Actor%20Object%20Reference) (OtherComp :type Primitive%20Component%20Object%20Reference) (OtherBodyIndex :type Integer) (bFromSweep :type Boolean) (SweepResult :type Hit%20Result%20Structure%20%28by%20ref%29))
  (bind _box (Variables|Default|GetBox))
  ;[1 1 1] Toggle on object overlap of any kind
  (bind _outactors (Class|KismetSystemLibrary|ComponentOverlapActorsNEW _box (Transformation|GetWorldTransform _box) (Utilities|Array|MakeArray "ObjectTypeQuery4" "ObjectTypeQuery2" "ObjectTypeQuery3" "ObjectTypeQuery6") "/Script/Engine.Actor" (Utilities|Array|MakeArray self)))
  (if (> (Utilities|Array|Length _outactors) 0)
    (if (not (Variables|Default|GetIsActive))
      (CallFunction|Toggle))
    (elif (Variables|Default|GetIsActive)
      (CallFunction|Toggle))))

(event OnComponentEndOverlap(Box)
  (params (OtherActor :type Actor%20Object%20Reference) (OtherComp :type Primitive%20Component%20Object%20Reference) (OtherBodyIndex :type Integer))
  (bind _box (Variables|Default|GetBox))
  ;[1 1 1] Toggle on object overlap of any kind
  (bind _outactors (Class|KismetSystemLibrary|ComponentOverlapActorsNEW _box (Transformation|GetWorldTransform _box) (Utilities|Array|MakeArray "ObjectTypeQuery4" "ObjectTypeQuery2" "ObjectTypeQuery3" "ObjectTypeQuery6") "/Script/Engine.Actor" (Utilities|Array|MakeArray self)))
  (if (> (Utilities|Array|Length _outactors) 0)
    (if (not (Variables|Default|GetIsActive))
      (CallFunction|Toggle))
    (elif (Variables|Default|GetIsActive)
      (CallFunction|Toggle))))

(event EventActivate
  ;[1 1 1] Push plate down a bit when it's toggle
  (if (Variables|Default|GetIsActive)
    (Transformation|SetActorLocation (+ (Variables|Default|GetInitial%20Location) (Math|Vector|MakeVector 0.0 0.0 -2.5)) false true)
    (else
      (Transformation|SetActorLocation (Variables|Default|GetInitial%20Location) false true))))

(event EventBeginPlay
  ;[1 1 1] Grab starting location for relative pressing
  (Variables|Default|SetInitial%20Location (Transformation|GetActorLocation)))

(fn ConstructionScript
  (|CallParentFunction))