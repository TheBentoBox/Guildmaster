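; Activatable door that slides from its starting location by a move offset, driven by an open timeline.
; On Activate, it opens only if it and every object in its query list are active; otherwise it reverses the timeline if closing is allowed.
; BeginPlay caches the start location and triggers Activate when the door starts active.
; A play-sound node exists but is unconnected.
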(event EventActivate
  ;[1 1 1] Listens for code event and plays open/close timeline
  (Variables|Default|SetAll%20Active true)
  (bind _array_element (Utilities|Array|ForEachLoopwithBreak (Variables|Default|GetObjects%20To%20Query))
    (:LoopBody
      (if (not (Variables|/Game/Blueprints/BP_Activatable.BP_Activatable_C|GetIsActive _array_element))
        (Variables|Default|SetAll%20Active (Variables|/Game/Blueprints/BP_Activatable.BP_Activatable_C|GetIsActive _array_element))))
    (:Completed
      (if (and (Variables|Default|GetAll%20Active) (Variables|Default|GetIsActive))
        (bind _open_amount (Timeline|Door%20Open%20Timeline Play)
          (:Update
            (Transformation|SetActorLocation (+ (* (Variables|Default|GetMove%20Offset) _open_amount) (Variables|Default|GetInitial%20Location)) false false)))
        (elif (Variables|Default|GetCan%20Close%20Once%20Opened)
          (Timeline|Door%20Open%20Timeline Reverse))))))

(event EventBeginPlay
  ;[1 1 1] Grab initial rotation for relative swing animation
  (Variables|Default|SetInitial%20Location (Transformation|GetActorLocation))
  (if (Variables|Default|GetIsActive)
    (CallFunction|Activate)))

(fn ConstructionScript
  (|CallParentFunction))