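; BP_Activatable is a base for lockable objects that switch between active and inactive and can trigger other activatables.
; Toggle prints a message if locked; otherwise it flips IsActive and calls Activate, which is empty here.
; It then walks ActivatesNext, toggling each target recursively.
; In IsSetter mode it instead forces targets to SetBool and calls Activate directly, bypassing their locks and further chaining.
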(event EventBeginPlay)

(event EventActorBeginOverlap
  (params (OtherActor :type Actor%20Object%20Reference)))

(event EventTick
  (params (DeltaSeconds :type Float%20%28single-precision%29)))

(fn ConstructionScript)

(fn Activate)

(fn Toggle
  ;[1 1 1] Toggles state, calls (de)activate and chains to ActivatesNext
  (if (Variables|Public|GetIsLocked)
    (Development|PrintString "It's locked.")
    (else
      (Variables|Public|SetIsActive (not (Variables|Public|GetIsActive)))
      (Interaction|Activate)
      (for _array_element (Variables|Interaction|GetActivatesNext)
        (Utilities|IsValid _array_element
          (:Is%20Valid
            (bind _asbp_activatable (Utilities|Casting|CastToBP_Activatable _array_element))
            (if (Variables|Public|GetIsSetter)
              (Variables|BP_Activatable_C|SetIsActive _asbp_activatable (Variables|Public|GetsetBool))
              (Interaction|Activate _asbp_activatable)
              (else
                (Interaction|Toggle _asbp_activatable)))))))))